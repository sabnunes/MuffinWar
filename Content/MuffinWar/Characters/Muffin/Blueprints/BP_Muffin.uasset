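; BP_Muffin is an AI-controlled muffin character that kills other muffins on contact with its attack hitbox.
; DoAttack toggles the hitbox between query-only and no collision, playing the attack sound when switching it off.
; Overlapping another BP_Muffin calls that muffin's OnDeath, which runs once, disables its hitbox, stops its AI logic, then after a short delay destroys it with a pop sound.
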(event `self.Hitbox.OnComponentBeginOverlap`
  (params (OverlappedComponent :type "PrimitiveComponent Object Reference") (OtherActor :type "Actor Object Reference") (OtherComp :type "PrimitiveComponent Object Reference") (OtherBodyIndex :type Integer) (bFromSweep :type Boolean) (SweepResult :type "HitResult Structure (by ref)"))
  (bind _asbp_muffin (cast `/Game/MuffinWar/Characters/Muffin/Blueprints/BP_Muffin` OtherActor))
  (`self.OnDeath` _asbp_muffin))

(event `OnDeath`
  (if (not (`self.IsDead`))
    (`PrimitiveComponent.SetCollisionEnabled` (`self.Hitbox`) "NoCollision")
    (set `self.IsDead` true)
    (`BrainComponent.StopLogic` (`AIController.BrainComponent` (`AIBlueprintHelperLibrary.GetAIController` self)) "")
    (`KismetSystemLibrary.Delay` 1.5)
    (`self.K2_DestroyActor`)
    (`GameplayStatics.PlaySoundAtLocation` "/Game/MuffinWar/Audio/S_MuffinPop_Cue.S_MuffinPop_Cue" (`self.K2_GetActorLocation`) (struct) 1.0 1.0 0.0 null null null)))

(fn `DoAttack`
  (params (IsAttacking :type Boolean))
  (bind _hitbox (`self.Hitbox`))
  (if IsAttacking
    (`PrimitiveComponent.SetCollisionEnabled` _hitbox "QueryOnly")
    (else
      (`PrimitiveComponent.SetCollisionEnabled` _hitbox "NoCollision")
      (set `self.IsAttacking` false)
      (`GameplayStatics.PlaySoundAtLocation` "/Game/MuffinWar/Audio/S_Attack_Cue.S_Attack_Cue" (`self.K2_GetActorLocation`) (struct) 1.0 1.0 0.0 null null null))))

(fn `UserConstructionScript`)